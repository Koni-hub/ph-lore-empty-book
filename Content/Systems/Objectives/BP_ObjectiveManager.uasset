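; BP_ObjectiveManager tracks a list of objectives, the active one and whether all are completed.
; SetActiveObjective flags the entry matching an ID as active without deactivating the previous one.
; CompleteObjective marks the active objective completed, clears the reference and runs CheckAllCompleted.
; That check sets AllCompleted and calls OnObjectivesChanged only when every objective is done, with debug prints along the way.
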(event `self.ReceiveBeginPlay`
  (`KismetSystemLibrary.PrintString` "ObjectiveManager Ready"))

(fn `CheckAllCompleted`
  (for _array_element (`self.Objectives`)
    (if (== (`/Game/Systems/Objectives/DA_ObjectiveData.bIsCompleted` _array_element) false)
      (return)))
  (set `self.bAllCompleted` true)
  (`KismetSystemLibrary.PrintString` "All Objectives Complete!")
  (`self.OnObjectivesChanged`))

(fn `CompleteObjective`
  (bind _activeobjective (`self.ActiveObjective`))
  (`KismetSystemLibrary.PrintString` "Completing Objective")
  (`/Engine/EditorBlueprintResources/StandardMacros.IsValid` (`self.ActiveObjective`)
    (:`Is Valid`
      (set `/Game/Systems/Objectives/DA_ObjectiveData.bIsCompleted` true _activeobjective)
      (set `/Game/Systems/Objectives/DA_ObjectiveData.bIsActive` false _activeobjective)
      (set `self.ActiveObjective` null)
      (`self.CheckAllCompleted`)
      (`KismetSystemLibrary.PrintString` "Going to All Completed"))))

(fn `SetActiveObjective`
  (params (`ObjectiveID ` :type Name))
  (for _array_element (`self.Objectives`)
    (if (== (`/Game/Systems/Objectives/DA_ObjectiveData.ObjectiveID` _array_element) `ObjectiveID `)
      (set `/Game/Systems/Objectives/DA_ObjectiveData.bIsActive` true _array_element)
      (set `self.ActiveObjective` _array_element))))

(fn `UserConstructionScript`)