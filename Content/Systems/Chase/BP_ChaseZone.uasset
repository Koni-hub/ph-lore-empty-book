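; BP_ChaseZone is a chase-zone actor that runs line-of-sight detection of Marco from Alan.
; While the zone is active with Marco inside, Tick traces between them; a Marco hit plays a one-time sound and updates SightMeter.
; That update clamps to the meter's current value, so it cannot rise as wired; otherwise, outside those conditions, it drains.
; BeginPlay caches BP_ChaseDirector, unused here.
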(event `self.ReceiveBeginPlay`
  (bind _outactors (`GameplayStatics.GetAllActorsOfClass` "/Game/Systems/Chase/BP_ChaseDirector.BP_ChaseDirector_C"))
  (set `self.ChaseDirectorReference` (`|GetArrayItem` _outactors))
  (`KismetSystemLibrary.PrintString` "ChaseZone Ready"))

(event `self.ReceiveTick`
  (params (DeltaSeconds :type "Float (single-precision)"))
  ; Advance Detection System
  (if (and (`self.bZoneActive`) (`self.bMarcoInZone`))
    (bind _outhit (`KismetSystemLibrary.LineTraceSingle` :`Start` (`self.K2_GetActorLocation` (`self.AlanReference`)) :`End` (`self.K2_GetActorLocation` (`self.MarcoReference`)) :`TraceChannel` "TraceTypeQuery1" :`DrawDebugType` "ForDuration"))
    (cast `/Game/Characters/Marco/Blueprints/BP_Marco_Character` (`.HitActor` (`GameplayStatics.BreakHitResult` _outhit)))
    (bind _output_get (set `self.bHasLineOfSight` true))
    (if _output_get
      (set `self.SightMeter` (`KismetMathLibrary.FClamp` (+ (`self.SightMeter`) (* (`self.SightFillRate`) DeltaSeconds)) 0.0 (`self.SightMeter`)))
      (if (not (`self.bSightSoundPlaying`))
        (`GameplayStatics.PlaySoundAtLocation` "/Engine/VREditor/Sounds/VR_shep_scale_up_01.VR_shep_scale_up_01" (`self.K2_GetActorLocation`) (struct) 1.0 1.0 0.0 null null null null)
        (set `self.bSightSoundPlaying` true)))
    (else
      (set `self.SightMeter` (`KismetMathLibrary.FClamp` (- (`self.SightMeter`) (* (`self.SightDrainRate`) DeltaSeconds)) 0.0 (`self.SightMeterMax`))))))

(fn `UserConstructionScript`)