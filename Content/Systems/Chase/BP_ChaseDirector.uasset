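; BP_ChaseDirector manages the state of a phased chase involving Alan and the player character, Marco.
; On BeginPlay it caches the first BP_Alan_Base in the level and the player's BP_Marco_Character.
; BeginChase activates Alan, and AdvanceChasePhase increments the phase until the maximum triggers EndChase, which resets state and stops him.
; PauseChase stops Alan only when ChasePaused is already true; nothing here sets that flag or resumes.
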(event `self.ReceiveBeginPlay`
  (bind _outactors (`GameplayStatics.GetAllActorsOfClass` "/Game/Characters/Creatures/Alan/Blueprints/BP_Alan_Base.BP_Alan_Base_C"))
  (set `self.AlanReference` (`|GetArrayItem` _outactors))
  (bind _asbp_marco_character (cast `/Game/Characters/Marco/Blueprints/BP_Marco_Character` (`GameplayStatics.GetPlayerCharacter` 0)))
  (set `self.MarcoReference` _asbp_marco_character)
  (`KismetSystemLibrary.PrintString` "ChaseDirector Initialized"))

(fn `AdvanceChasePhase`
  (if (`self.bChaseActive`)
    (set `self.ChasePhase` (+ (`self.ChasePhase`) 1))
    (if (>= (`self.ChasePhase`) (`self.MaxChasePhases`))
      (`self.EndChase`)
      (else
        (`KismetSystemLibrary.PrintString` "Chase Phase Advanced")))))

(fn `BeginChase`
  (if (not (`self.bChaseActive`))
    (set `self.bChaseActive` true)
    (set `self.ChasePhase` 0)
    (if (`KismetSystemLibrary.IsValid` (`self.AlanReference`))
      (`/Game/Characters/Creatures/Alan/Blueprints/BP_Alan_Base.ActivateAlan` (`self.AlanReference`))
      (`KismetSystemLibrary.PrintString` "Chase Begun"))))

(fn `EndChase`
  (set `self.bChaseActive` false)
  (set `self.ChasePhase` 0)
  (if (`KismetSystemLibrary.IsValid` (`self.AlanReference`))
    (`/Game/Characters/Creatures/Alan/Blueprints/BP_Alan_Base.StopChase` (`self.AlanReference`))
    (`KismetSystemLibrary.PrintString` "Chase Ended")))

(fn `PauseChase`
  (if (`self.bChasePaused`)
    (if (`KismetSystemLibrary.IsValid` (`self.AlanReference`))
      (`/Game/Characters/Creatures/Alan/Blueprints/BP_Alan_Base.StopChase` (`self.AlanReference`))
      (`KismetSystemLibrary.PrintString` "Chase Paused"))))

(fn `UserConstructionScript`)