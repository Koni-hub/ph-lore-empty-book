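; BP_DialogueManager is a dialogue manager that starts and ends conversations, currently showing lines as debug prints.
; PlayConversation stores the given conversation, resets the line index, then calls ShowNextLine to print that line's speaker and text.
; ShowNextLine calls EndConversation to clear state once the index passes the last line, but nothing here increments the index.
; BeginPlay caches the player's BP_Marco_Character, which is otherwise unused here.
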(event `self.ReceiveBeginPlay`
  (bind _asbp_marco_character (cast `/Game/Characters/Marco/Blueprints/BP_Marco_Character` (`GameplayStatics.GetPlayerCharacter` 0)))
  (set `self.MarcoReference` _asbp_marco_character)
  (`KismetSystemLibrary.PrintText` "DialogueManager Ready"))

(fn `EndConversation`
  (set `self.bIsPlaying` false)
  (set `self.CurrentLineIndex` 0)
  (set `self.CurrentConversation   ` null)
  (`KismetSystemLibrary.PrintText` "Dialogue Ended"))

(fn `PlayConversation`
  (params (`Conversation ` :type "/Game/Systems/Dialogue/DialgoueConversation/DA_DialogueConversation Object Reference"))
  (set `self.CurrentConversation   ` `Conversation `)
  (set `self.CurrentLineIndex` 0)
  (set `self.bIsPlaying` true)
  (`self.ShowNextLine`))

(fn `ShowNextLine`
  (bind _output (`|GetArrayItem` (`/Game/Systems/Dialogue/DialgoueConversation/DA_DialogueConversation.DialogueLines` (`self.CurrentConversation   `)) (`self.CurrentLineIndex`)))
  (if (< (`self.CurrentLineIndex`) (`KismetArrayLibrary.Array_Length` (`/Game/Systems/Dialogue/DialgoueConversation/DA_DialogueConversation.DialogueLines` (`self.CurrentConversation   `))))
    (`KismetSystemLibrary.PrintString` (`KismetTextLibrary.Conv_TextToString` (`|FormatText` "Speaker Name: {speaker} \n{dialog}" (`/Game/Systems/Dialogue/DialogueLines/DA_DialogueLine.SpeakerName` _output) (`/Game/Systems/Dialogue/DialogueLines/DA_DialogueLine.DialogueText` _output))))
    (else
      (`self.EndConversation`))))

(fn `UserConstructionScript`)