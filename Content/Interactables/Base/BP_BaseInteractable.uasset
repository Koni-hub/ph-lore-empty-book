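; Base interactable actor that the player can hover and interact with, meant as a parent for specific interactables.
; A sphere overlap with the player character notifies the player's InteractionComponent when it enters or leaves range.
; Hover events toggle the tooltip and a custom-depth stencil outline on the mesh.
; Interact only prints a debug string, and GetInvestigationNode is an empty stub.
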(event `self.Sphere.OnComponentBeginOverlap`
  (params (OverlappedComponent :type "PrimitiveComponent Object Reference") (OtherActor :type "Actor Object Reference") (OtherComp :type "PrimitiveComponent Object Reference") (OtherBodyIndex :type Integer) (bFromSweep :type Boolean) (SweepResult :type "HitResult Structure (by ref)"))
  (bind _returnvalue (`self.GetComponentByClass` OtherActor "/Game/Interactables/Base/InteractionComponent.InteractionComponent_C"))
  ; Begin/End Overlap
  (if (== OtherActor (`GameplayStatics.GetPlayerCharacter` 0))
    (if (`KismetSystemLibrary.IsValid` _returnvalue)
      (`/Game/Interactables/Base/InteractionComponent.On Interactable Overlap` _returnvalue true))))

(event `self.Sphere.OnComponentEndOverlap`
  (params (OverlappedComponent :type "PrimitiveComponent Object Reference") (OtherActor :type "Actor Object Reference") (OtherComp :type "PrimitiveComponent Object Reference") (OtherBodyIndex :type Integer))
  (bind _returnvalue (`self.GetComponentByClass` OtherActor "/Game/Interactables/Base/InteractionComponent.InteractionComponent_C"))
  ; Begin/End Overlap
  (if (== OtherActor (`GameplayStatics.GetPlayerCharacter` 0))
    (if (`KismetSystemLibrary.IsValid` _returnvalue)
      (`/Game/Interactables/Base/InteractionComponent.On Interactable Overlap` _returnvalue false))))

(event `/Game/Interactables/Base/BPI_Interactable.On Hovered`
  ; Hovered/UnHovered
  (`SceneComponent.SetVisibility` (`self.ToolTip`) true false)
  (`self.Highlight Outline` true))

(event `/Game/Interactables/Base/BPI_Interactable.On UnHovered`
  ; Hovered/UnHovered
  (`SceneComponent.SetVisibility` (`self.ToolTip`) false false)
  (`self.Highlight Outline` false))

(event `Highlight Outline`
  (params (Show :type Boolean))
  (bind _interactable_mesh (`self.Interactable Mesh`))
  ; Highlight Object Outline
  (`PrimitiveComponent.SetRenderCustomDepth` _interactable_mesh Show)
  (`PrimitiveComponent.SetCustomDepthStencilValue` _interactable_mesh (select `bool` Show :`true` 2)))

(event `/Game/Interactables/Base/BPI_Interactable.Interact`
  (params (Character :type "Actor Object Reference"))
  ; Interact
  (`KismetSystemLibrary.PrintString` "Interacting"))

(fn `GetInvestigationNode`
  (returns (Node :type "/Game/Systems/Investigation/DA_InvestigationNode Object Reference"))
  (return null))

(fn `UserConstructionScript`)