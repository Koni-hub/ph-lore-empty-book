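; Base interactable that lets the player inspect an object up close through a WBP_Inspect widget.
; The construction script copies InteractableMesh into InspectableMesh at relative Z -1000, with a show-only SceneCaptureComponent2D for isolated capture.
; Interact reveals the copy, opens the UI and switches BP_PlayerController_Marco to inspect input.
; Events rotate, pan within clamped bounds and zoom via capture FOV; exiting resets the copy and restores gameplay input.
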(event `/Game/Interactables/Base/BPI_Interactable.Interact`
  (params (Character :type "Actor Object Reference"))
  (bind _returnvalue (`GameplayStatics.GetPlayerController` 0))
  (bind _scenecapturecomponent2d (`self.SceneCaptureComponent2D`))
  ; Interact
  (`SceneCaptureComponent.SetCaptureSortPriority` _scenecapturecomponent2d 0)
  (`SceneComponent.SetVisibility` _scenecapturecomponent2d true false)
  (`SceneComponent.SetHiddenInGame` (`self.Inspectable Mesh`) false false)
  (bind _returnvalue_2 (`|CreateWidget` "/Game/UI/Interact/WBP_Inspect.WBP_Inspect_C"))
  (bind _output_get (set `self.Inspect UI` _returnvalue_2))
  (set `/Game/UI/Interact/WBP_Inspect.InspectData ` (`self.DA_InspectData`) _output_get)
  (`UserWidget.AddToViewport` _output_get 0)
  (set `PlayerController.bShowMouseCursor` true _returnvalue)
  (`WidgetBlueprintLibrary.SetInputMode_GameAndUIEx` _returnvalue null)
  (bind _asbp_player_controller_marco (cast `/Game/Characters/Marco/Blueprints/BP_PlayerController_Marco` (`GameplayStatics.GetPlayerController` 0))
    (:`then`
      (`/Game/Characters/Marco/Blueprints/BP_PlayerController_Marco.Update Input Max Context` _asbp_player_controller_marco "/Game/Interactables/Base/InspectInput/IMC_Inspect.IMC_Inspect")
      (set `/Game/Characters/Marco/Blueprints/BP_PlayerController_Marco.Inspectable BP` self _asbp_player_controller_marco))
    (:`CastFailed`
      (`KismetSystemLibrary.PrintString` "Not Controller?"))))

(event `Update Mesh Zoom`
  (params (Axis :type "Float (double-precision)"))
  ; Zoom In/Out
  (set `SceneCaptureComponent2D.FOVAngle` (`KismetMathLibrary.FClamp` (+ (* Axis -3.0) (`SceneCaptureComponent2D.FOVAngle` (`self.SceneCaptureComponent2D`))) 10.0 120.0) (`self.SceneCaptureComponent2D`)))

(event `Update Mesh Rotation`
  (params (`Vector 2D` :type "Vector2D Structure"))
  (bind (_x _y) (`KismetMathLibrary.BreakVector2D` `Vector 2D`))
  (bind _inspectable_mesh (`self.Inspectable Mesh`))
  ; Mouse Rotation (X/Z)
  (`SceneComponent.K2_SetRelativeRotation` _inspectable_mesh (`KismetMathLibrary.ComposeRotators` (`SceneComponent.RelativeRotation` _inspectable_mesh) (`KismetMathLibrary.MakeRotator` (* _y -5.0) 0.0 (* _x -5.0))) false false))

(event `Exit Inspect Mode`
  (bind _returnvalue (`GameplayStatics.GetPlayerController` 0))
  ; Exit Inspect
  (`self.Reset Inspectable Mesh`)
  (`SceneComponent.SetHiddenInGame` (`self.Inspectable Mesh`) true false)
  (`SceneComponent.SetHiddenInGame` (`self.SceneCaptureComponent2D`) false false)
  (`Widget.RemoveFromParent` (`self.Inspect UI`))
  (set `PlayerController.bShowMouseCursor` false _returnvalue)
  (`WidgetBlueprintLibrary.SetInputMode_GameOnly` _returnvalue)
  (bind _asbp_player_controller_marco (cast `/Game/Characters/Marco/Blueprints/BP_PlayerController_Marco` (`GameplayStatics.GetPlayerController` 0)))
  (`/Game/Characters/Marco/Blueprints/BP_PlayerController_Marco.Update Input Max Context` _asbp_player_controller_marco "/Game/Characters/Marco/Input/IMC_Marco.IMC_Marco"))

(event `Reset Inspectable Mesh`
  (bind _scenecapturecomponent2d (`self.SceneCaptureComponent2D`))
  ; Reset Inspectable Mesh
  (`SceneComponent.K2_SetRelativeTransform` (`self.Inspectable Mesh`) (`self.Inspectable Default Value`) false false)
  (set `SceneCaptureComponent2D.FOVAngle` 90.0 (`self.SceneCaptureComponent2D`))
  (`SceneCaptureComponent.SetCaptureSortPriority` _scenecapturecomponent2d 1)
  (`SceneComponent.SetVisibility` _scenecapturecomponent2d false false))

(event `Update Mesh Location`
  (params (Vector2D :type "Vector2D Structure"))
  (bind (_x _y) (`KismetMathLibrary.BreakVector2D` Vector2D))
  (bind _inspectable_mesh (`self.Inspectable Mesh`))
  (bind (_relativelocation_x _relativelocation_y _relativelocation_z) (`KismetMathLibrary.BreakVector` (`SceneComponent.RelativeLocation` (`self.Inspectable Mesh`))))
  (bind _relativelocation_x_2 (`KismetMathLibrary.BreakVector` (`SceneComponent.RelativeLocation` _inspectable_mesh)))
  (bind _x_2 (.x (.location (`self.Inspectable Default Value`))))
  (bind _z (.z (.location (`self.Inspectable Default Value`))))
  ; Mouse Move  Object (X./Z)
  (`SceneComponent.K2_SetRelativeLocation` _inspectable_mesh (`KismetMathLibrary.MakeVector` (`KismetMathLibrary.FClamp` (+ _relativelocation_x_2 (* _x 2.0)) (- _x_2 100.0) (+ _x_2 100.0)) 0.0 (`KismetMathLibrary.FClamp` (+ _relativelocation_z (* _y 2.0)) (- _z 100.0) (+ _z 100.0))) false false))

(fn `UserConstructionScript`
  (bind _inspectable_mesh (`self.Inspectable Mesh`))
  (bind _scenecapturecomponent2d (`self.SceneCaptureComponent2D`))
  (bind _interactable_mesh (`self.Interactable Mesh`))
  (bind _inspectable_mesh_2 (`self.Inspectable Mesh`))
  (bind (_relativelocation_x _relativelocation_y) (`KismetMathLibrary.BreakVector` (`SceneComponent.RelativeLocation` _scenecapturecomponent2d)))
  (bind (_relativelocation_x_2 _relativelocation_y_2) (`KismetMathLibrary.BreakVector` (`SceneComponent.RelativeLocation` _inspectable_mesh_2)))
  (`parent.UserConstructionScript`)
  (`SceneCaptureComponent.ShowOnlyComponent` (`self.SceneCaptureComponent2D`) (`self.Inspectable Mesh`))
  (`PrimitiveComponent.SetMaterial` _inspectable_mesh 0 (`PrimitiveComponent.GetMaterial` (`self.Interactable Mesh`) 0))
  (`StaticMeshComponent.SetStaticMesh` _inspectable_mesh (`StaticMeshComponent.StaticMesh` _interactable_mesh))
  (`SceneComponent.K2_SetRelativeTransform` _inspectable_mesh (`SceneComponent.GetRelativeTransform` _interactable_mesh) false false)
  (`SceneComponent.K2_SetRelativeLocation` _inspectable_mesh_2 (`KismetMathLibrary.MakeVector` _relativelocation_x_2 _relativelocation_y_2 -1000.0) false false)
  (`SceneComponent.K2_SetRelativeLocation` _scenecapturecomponent2d (`KismetMathLibrary.MakeVector` _relativelocation_x _relativelocation_y -1000.0) false false)
  (set `self.Inspectable Default Value` (`SceneComponent.GetRelativeTransform` (`self.Inspectable Mesh`))))