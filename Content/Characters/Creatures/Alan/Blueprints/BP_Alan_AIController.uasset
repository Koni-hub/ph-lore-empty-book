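; AI controller for the Alan creature that runs its behavior tree and triggers a chase of Marco.
; On possession it caches the Alan pawn; perception updates set that pawn's CanSeeMarco flag for Marco.
; It binds to the first chase zone's sight-meter-full event, which starts the chase and writes a Chasing state to the blackboard.
; A helper function also writes Marco's location to the blackboard.
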(event `self.ReceiveBeginPlay`
  (bind _outactors (`GameplayStatics.GetAllActorsOfClass` "/Game/Systems/Chase/BP_ChaseZone.BP_ChaseZone_C"))
  (bind _output_get (set `self.ChaseZoneReference` (`|GetArrayItem` _outactors)))
  (add `/Game/Systems/Chase/BP_ChaseZone.OnSightMeterFull` _output_get (delegate `OnDetectionFull`)))

(event `OnDetectionFull`
  (`KismetSystemLibrary.PrintString` "Detection is Full Start Chasing")
  (`/Game/Characters/Creatures/Alan/Blueprints/BP_Alan_Base.StartChase` (`self.AlanReference`))
  (`self.UpdateAlanState` "Chasing")
  (`KismetSystemLibrary.PrintString` "Chase Started – Detection Full!"))

(event `self.ReceivePossess`
  (params (PossessedPawn :type "Pawn Object Reference"))
  (bind _asbp_alan_base (cast `/Game/Characters/Creatures/Alan/Blueprints/BP_Alan_Base` PossessedPawn))
  (set `self.AlanReference` _asbp_alan_base)
  (`self.RunBehaviorTree` "/Game/Characters/Creatures/Alan/AI/BT_Alan.BT_Alan"))

(event `self.AIPerception.OnTargetPerceptionUpdated`
  (params (Actor :type "Actor Object Reference") (Stimulus :type "AIStimulus Structure"))
  (bind _alanreference (`self.AlanReference`))
  (cast `/Game/Characters/Marco/Blueprints/BP_Marco_Character` Actor)
  (if (`.bSuccessfullySensed` (break `AIStimulus` Stimulus))
    (set `/Game/Characters/Creatures/Alan/Blueprints/BP_Alan_Base.bCanSeeMarco` true _alanreference)
    (else
      (set `/Game/Characters/Creatures/Alan/Blueprints/BP_Alan_Base.bCanSeeMarco` false _alanreference))))

(fn `UpdateAlanState`
  (params (NewState :type Name))
  (`BlackboardComponent.SetValueAsName` (`AIBlueprintHelperLibrary.GetBlackboard` null) "AlanState" NewState))

(fn `UpdateMarcoLocation`
  (`BlackboardComponent.SetValueAsVector` (`AIBlueprintHelperLibrary.GetBlackboard` null) "MarcoLocation" (`self.K2_GetActorLocation` (`/Game/Characters/Creatures/Alan/Blueprints/BP_Alan_Base.MarcoReference` (`self.AlanReference`)))))

(fn `UserConstructionScript`)