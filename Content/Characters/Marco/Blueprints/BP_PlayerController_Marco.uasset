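; Player controller for Marco that handles pause, journal and object-inspection input through Enhanced Input.
; A custom event swaps the active mapping context at runtime by clearing all mappings and adding the new one.
; Inspect actions forward mouse wheel zoom, left-drag rotation, right-drag movement and exit to InspectableBP, using click flags to gate mouse movement.
; Pause sets the game paused, while the journal toggle only flips a flag and prints placeholder text.
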(event `Update Input Max Context`
  (params (MappingContext :type "InputMappingContext Object Reference"))
  (bind _returnvalue (subsystem `EnhancedInputLocalPlayerSubsystem`))
  ; Update Input Mapping Context at Runtime
  (`/Engine/EditorBlueprintResources/StandardMacros.IsValid` _returnvalue
    (:`Is Valid`
      (`EnhancedInputSubsystemInterface.ClearAllMappings` _returnvalue)
      (`EnhancedInputSubsystemInterface.AddMappingContext` _returnvalue MappingContext 0 (struct)))))

(event `EnhancedInput|/Game/Characters/Marco/Input/IA_Pause`
  (params (ActionValue :type Boolean) (ElapsedSeconds :type "Float (double-precision)") (TriggeredSeconds :type "Float (double-precision)") (InputAction :type "InputAction Object Reference" :default "/Game/Characters/Marco/Input/IA_Pause.IA_Pause"))
  ;[0.15 0.15 1 0.5] Pause Input
  (:`Started`
    (`GameplayStatics.SetGamePaused` true)
    (`KismetSystemLibrary.PrintString` "Game Paused")))

(event `EnhancedInput|/Game/Characters/Marco/Input/IA_OpenJournal`
  (params (ActionValue :type Boolean) (ElapsedSeconds :type "Float (double-precision)") (TriggeredSeconds :type "Float (double-precision)") (InputAction :type "InputAction Object Reference" :default "/Game/Characters/Marco/Input/IA_OpenJournal.IA_OpenJournal"))
  ;[0.15 0.15 1 0.5] Journal Input
  (:`Started`
    (if (`self.bJournalOpen`)
      (set `self.bJournalOpen` false)
      (`KismetSystemLibrary.PrintString` "[Hide Journal UI]")
      (else
        (set `self.bJournalOpen` true)
        (`KismetSystemLibrary.PrintString` "[Show Journal UI]")))))

(event `EnhancedInput|/Game/Interactables/Base/InspectInput/AI_MouseWheel`
  (params (ActionValue :type "Float (double-precision)") (ElapsedSeconds :type "Float (double-precision)") (TriggeredSeconds :type "Float (double-precision)") (InputAction :type "InputAction Object Reference" :default "/Game/Interactables/Base/InspectInput/AI_MouseWheel.AI_MouseWheel"))
  ;[0.15 1 0.15 0.5] Mouse Wheel (Zoom In/Out)
  (:`Triggered`
    (`/Game/Interactables/Base/BP_Inspectable.Update Mesh Zoom` (`self.Inspectable BP`) ActionValue)))

(event `EnhancedInput|/Game/Interactables/Base/InspectInput/AI_LeftMouse`
  (params (ActionValue :type Boolean) (ElapsedSeconds :type "Float (double-precision)") (TriggeredSeconds :type "Float (double-precision)") (InputAction :type "InputAction Object Reference" :default "/Game/Interactables/Base/InspectInput/AI_LeftMouse.AI_LeftMouse"))
  ;[0.15 1 0.15 0.5] Left Mouse/Right Mouse Click
  (:`Started`
    (set `self.LeftClick Active` true))
  (:`Completed`
    (set `self.LeftClick Active` false)))

(event `EnhancedInput|/Game/Interactables/Base/InspectInput/AI_RightMouse`
  (params (ActionValue :type Boolean) (ElapsedSeconds :type "Float (double-precision)") (TriggeredSeconds :type "Float (double-precision)") (InputAction :type "InputAction Object Reference" :default "/Game/Interactables/Base/InspectInput/AI_RightMouse.AI_RightMouse"))
  ;[0.15 1 0.15 0.5] Left Mouse/Right Mouse Click
  (:`Started`
    (set `self.RightClick Active` true))
  (:`Completed`
    (set `self.RightClick Active` false)))

(event `EnhancedInput|/Game/Interactables/Base/InspectInput/AI_MouseMove`
  (params (ActionValue :type "Vector2D Structure") (ElapsedSeconds :type "Float (double-precision)") (TriggeredSeconds :type "Float (double-precision)") (InputAction :type "InputAction Object Reference" :default "/Game/Interactables/Base/InspectInput/AI_MouseMove.AI_MouseMove"))
  ;[0.15 1 0.15 0.5] Mouse Moving
  (:`Triggered`
    (`|ExecutionSequence`
      (:`then_0`
        (if (`self.LeftClick Active`)
          (`/Game/Interactables/Base/BP_Inspectable.Update Mesh Rotation` (`self.Inspectable BP`) ActionValue)))
      (:`then_1`
        (if (`self.RightClick Active`)
          (`/Game/Interactables/Base/BP_Inspectable.Update Mesh Location` (`self.Inspectable BP`) ActionValue))))))

(event `EnhancedInput|/Game/Interactables/Base/InspectInput/AI_ExitInspectMode`
  (params (ActionValue :type Boolean) (ElapsedSeconds :type "Float (double-precision)") (TriggeredSeconds :type "Float (double-precision)") (InputAction :type "InputAction Object Reference" :default "/Game/Interactables/Base/InspectInput/AI_ExitInspectMode.AI_ExitInspectMode"))
  (:`Started`
    (`/Game/Interactables/Base/BP_Inspectable.Exit Inspect Mode` (`self.Inspectable BP`))))

(fn `UserConstructionScript`)